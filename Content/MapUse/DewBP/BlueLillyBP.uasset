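; Blue lily actor that marks the player's BP_TesterCharacter as holding dew while it overlaps the Capsule.
; BeginPlay creates and stores a ConsumingDews widget, without adding it to the viewport here.
; Begin overlap sets HoldingDew on the character; end overlap clears it, prints a debug string and resets the widget's TimeHeld.
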(event OnComponentBeginOverlap(Capsule)
  (params (OverlappedComponent :type Primitive%20Component%20Object%20Reference) (OtherActor :type Actor%20Object%20Reference) (OtherComp :type Primitive%20Component%20Object%20Reference) (OtherBodyIndex :type Integer) (bFromSweep :type Boolean) (SweepResult :type Hit%20Result%20Structure%20%28by%20ref%29))
  (bind _asbp_tester_character (Utilities|Casting|CastToBP_TesterCharacter OtherActor))
  (bind _output_get (Variables|Default|SetAs%20BP%20Tester%20Character _asbp_tester_character))
  (Variables|/Game/MapUse/BP_TesterCharacter.BP_TesterCharacter_C|SetHoldingDew _output_get true))

(event OnComponentEndOverlap(Capsule)
  (params (OverlappedComponent :type Primitive%20Component%20Object%20Reference) (OtherActor :type Actor%20Object%20Reference) (OtherComp :type Primitive%20Component%20Object%20Reference) (OtherBodyIndex :type Integer))
  (bind _asbp_tester_character (Utilities|Casting|CastToBP_TesterCharacter OtherActor))
  (bind _output_get (Variables|Default|SetAs%20BP%20Tester%20Character_0 _asbp_tester_character))
  (Variables|/Game/MapUse/BP_TesterCharacter.BP_TesterCharacter_C|SetHoldingDew _output_get false)
  (Development|PrintString "endoverlap")
  (Variables|/Game/MapUse/ConsumingWidget/ConsumingDews.ConsumingDews_C|SetTimeHeld (Variables|Default|GetConsumeWidget) 0.0))

(event EventBeginPlay
  (bind _returnvalue (UserInterface|CreateWidget "/Game/MapUse/ConsumingWidget/ConsumingDews.ConsumingDews_C"))
  (Variables|Default|SetConsumeWidget _returnvalue))

(event Collision|EventActorBeginOverlap
  (params (OtherActor :type Actor%20Object%20Reference)))

(event EventTick
  (params (DeltaSeconds :type Float%20%28single-precision%29)))

(fn ConstructionScript)