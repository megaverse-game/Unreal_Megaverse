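; Pilotable drone pawn that flags nearby BP_TesterCharacters for entry and, once landed, lets the player exit into a newly spawned character.
; Upward input sets InAir, enabling lerp-smoothed movement, turning and speed boost, while Cube overlap lands it and enables exit.
; Tick tilts the mesh with input or adds random idle wobble.
; Hard strafing temporarily detaches spring-arm control rotation to swing the camera toward the drone.
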(event OnComponentBeginOverlap(Box)
  (params (OverlappedComponent :type Primitive%20Component%20Object%20Reference) (OtherActor :type Actor%20Object%20Reference) (OtherComp :type Primitive%20Component%20Object%20Reference) (OtherBodyIndex :type Integer) (bFromSweep :type Boolean) (SweepResult :type Hit%20Result%20Structure%20%28by%20ref%29))
  (Utilities|FlowControl|Sequence
    (:then_0
      (bind _asbp_tester_character (Utilities|Casting|CastToBP_TesterCharacter OtherActor))
      (Variables|/Game/MapUse/BP_TesterCharacter.BP_TesterCharacter_C|SetDroneEnter _asbp_tester_character true)
      (Development|PrintString "Droneenter"))))

(event OnComponentEndOverlap(Box)
  (params (OverlappedComponent :type Primitive%20Component%20Object%20Reference) (OtherActor :type Actor%20Object%20Reference) (OtherComp :type Primitive%20Component%20Object%20Reference) (OtherBodyIndex :type Integer))
  (bind _asbp_tester_character (Utilities|Casting|CastToBP_TesterCharacter OtherActor))
  (Variables|/Game/MapUse/BP_TesterCharacter.BP_TesterCharacter_C|SetDroneEnter _asbp_tester_character false)
  (Development|PrintString "DroneExit"))

(event OnComponentBeginOverlap(Cube)
  (params (OverlappedComponent :type Primitive%20Component%20Object%20Reference) (OtherActor :type Actor%20Object%20Reference) (OtherComp :type Primitive%20Component%20Object%20Reference) (OtherBodyIndex :type Integer) (bFromSweep :type Boolean) (SweepResult :type Hit%20Result%20Structure%20%28by%20ref%29))
  (if (Variables|Default|GetInAir)
    (Development|PrintString "ppppp")
    (Variables|Default|SetInAir false)
    (Variables|Default|SetExitDrone true)))

(event EventBeginPlay
  (Variables|Default|SetPlayer (Pawn|GetControlledPawn (Game|GetPlayerController 0)))
  (bind _returnvalue (UserInterface|CreateWidget "/Game/MapUse/dewpercentage/DewPercentage.DewPercentage_C"))
  (Variables|Default|SetDewpercentWidgetBp _returnvalue))

(event Collision|EventActorBeginOverlap
  (params (OtherActor :type Actor%20Object%20Reference)))

(event EventTick
  (params (DeltaSeconds :type Float%20%28single-precision%29))
  (bind _returnvalue (Math|Random|RandomFloatinRange -7.0 7.0))
  (bind _returnvalue_2 (Transformation|GetActorRotation))
  (bind _returnvalue_3 (Math|Rotator|MakeRotator _returnvalue _returnvalue _returnvalue))
  (bind _returnvalue_4 (Math|Rotator|Lerp(Rotator) _returnvalue_2 _returnvalue_3 0.01))
  (if (Variables|Default|GetInAir)
    (if (Math|Boolean|ANDBoolean (== (Input|AxisValues|GetMoveup/Down) 0.0) (== (Input|AxisValues|GetMoveForward/Backward) 0.0) (== (Input|AxisValues|GetMoveRight/Left) 0.0) (< (Math|Float|Absolute(Float) (.yaw (Pawn|GetControlRotation :!class /Script/Engine.Pawn))) 1.0))
      (Development|PrintString "")
      (Utilities|FlowControl|DoOnce false :!label _label
        (:Completed
          (Development|PrintString "kello")
          (Components|MoveComponentTo (Variables|Default|GetMeshScene) "0, 0, 0" (Math|Rotator|MakeRotator (.roll _returnvalue_4) (.pitch _returnvalue_4) (.yaw _returnvalue_4)) true true 0.2 true)
          (goto _label Reset)))
      (else
        (Transformation|SetRelativeRotation (Variables|Default|GetMeshScene) (Math|Rotator|MakeRotator (* (Input|AxisValues|GetMoveRight/Left) (Math|Float|Lerp 1.0 4.0 0.01)) (* (Input|AxisValues|GetMoveForward/Backward) (Math|Float|Lerp -1.0 -4.0 0.01)) 0.0) false false)))))

(event Input|ActionEvents|InputActionSpeedupDrone
  (params (Key :type Key%20Structure :default "None"))
  (:Pressed
    (if (and (Variables|Default|GetBoostReady) (Variables|Default|GetInAir))
      (Development|PrintString "Works")
      (Variables|/Script/Engine.FloatingPawnMovement|SetMaxSpeed (Variables|Default|GetFloatingPawnMovement) 4e+03)
      (Variables|Default|SetBoostReady false)
      (Utilities|FlowControl|Delay 0.8)
      (Variables|Default|SetBoostReady true)))
  (:Released
    (Variables|/Script/Engine.FloatingPawnMovement|SetMaxSpeed (Variables|Default|GetFloatingPawnMovement) 1.2e+03)))

(event Input|AxisEvents|InputAxisTurnRight/LeftMouse
  (params (AxisValue :type Float%20%28single-precision%29))
  ;[0.05098 0.05098 0.05098] Camera Input - Mouse
  (Pawn|Input|AddControllerYawInput (* AxisValue 0.5)))

(event Input|AxisEvents|InputAxisLookUp/DownMouse
  (params (AxisValue :type Float%20%28single-precision%29))
  ;[0.05098 0.05098 0.05098] Camera Input - Mouse
  (Pawn|Input|AddControllerPitchInput (* AxisValue 0.5)))

(event Input|AxisEvents|InputAxisMoveForward/Backward
  (params (AxisValue :type Float%20%28single-precision%29))
  (if (Variables|Default|GetInAir)
    (bind _output_get (Variables|Default|SetForward (Math|Float|Lerp (Variables|Default|GetForward) AxisValue 0.01)))
    (Pawn|Input|AddMovementInput (Transformation|GetActorForwardVector) _output_get false)))

(event Input|AxisEvents|InputAxisMoveup/Down
  (params (AxisValue :type Float%20%28single-precision%29))
  (if (> AxisValue 0.0)
    (Variables|Default|SetInAir true)
    (Variables|Default|SetExitDrone false)
    (Development|PrintString ""))
  (Pawn|Input|AddMovementInput (Transformation|GetActorUpVector) (* AxisValue 0.5) false))

(event Input|AxisEvents|InputAxisTurninplace
  (params (AxisValue :type Float%20%28single-precision%29))
  (if (Variables|Default|GetInAir)
    (bind _output_get (Variables|Default|SetTurninplace (Math|Float|Lerp (Variables|Default|GetTurninplace) (Math|Float|SelectFloat AxisValue (Math|Float|Clamp(Float) (/ (.yaw (Math|Rotator|Delta(Rotator) (Pawn|GetControlRotation :!class /Script/Engine.Pawn) (Transformation|GetActorRotation))) 9e+01) -1.0) (> (Math|Float|Absolute(Float) AxisValue) 0.1)) 0.01)))
    (if (Variables|/Script/Engine.SpringArmComponent|GetbUsePawnControlRotation (Variables|Default|GetSpringArm))
      (Transformation|SetActorRotation (Math|Rotator|MakeRotator 0.0 0.0 (+ (.yaw (Transformation|GetActorRotation)) (* _output_get 0.8)))))))

(event Input|AxisEvents|InputAxisMoveRight/Left
  (params (AxisValue :type Float%20%28single-precision%29))
  (bind _returnvalue (Transformation|GetActorLocation))
  (bind _camera (Variables|Default|GetCamera))
  (bind _returnvalue_2 (Transformation|GetWorldLocation _camera))
  (bind _returnvalue_3 (Transformation|GetWorldRotation _camera))
  (bind _returnvalue_4 (Math|Rotator|FindLookatRotation _returnvalue_2 _returnvalue))
  (bind _returnvalue_5 (Math|Rotator|Lerp(Rotator) _returnvalue_3 _returnvalue_4 0.01))
  (if (Variables|Default|GetInAir)
    (bind _output_get (Variables|Default|SetRight (Math|Float|Lerp (Variables|Default|GetRight) AxisValue 0.01)))
    (if (> (Math|Float|Absolute(Float) (Variables|Default|GetRight)) 0.9)
      (Variables|/Script/Engine.SpringArmComponent|SetbUsePawnControlRotation (Variables|Default|GetSpringArm) false)
      (Pawn|SetControlRotation (Game|GetPlayerController 0) (Math|Rotator|MakeRotator 0.0 0.0 (.yaw _returnvalue_5)))
      (Transformation|SetWorldRotation _camera (Math|Rotator|MakeRotator 0.0 0.0 (.yaw _returnvalue_5)) false false)
      (Transformation|AddActorLocalRotation (Math|Rotator|MakeRotator 0.0 0.0 (Math|Float|Lerp (Variables|Default|GetRight) AxisValue 0.01)) false false)
      (Utilities|FlowControl|Delay 2.0)
      (Development|PrintString "Delay")
      (Variables|/Script/Engine.SpringArmComponent|SetbUsePawnControlRotation (Variables|Default|GetSpringArm) true)
      (else
        (Pawn|Input|AddMovementInput (Transformation|GetActorRightVector) _output_get false)))))

(event Input|KeyboardEvents|E
  (params (Key :type Key%20Structure :default "None"))
  (:Pressed
    (if (Variables|Default|GetExitDrone)
      (Development|PrintString "Cane")
      (bind _returnvalue (Game|SpawnActorfromClass "/Game/MapUse/BP_TesterCharacter.BP_TesterCharacter_C" (Math|Transform|MakeTransform (Transformation|GetWorldLocation (Variables|Default|GetExitPoint)) "0, 0, 0" "1.000000,1.000000,1.000000") "AlwaysSpawn" 0 0))
      (Pawn|Possess (Game|GetPlayerController 0) _returnvalue)
      (Rendering|SetVisibility (Variables|Default|GetEnterWidget) true false)
      (UserInterface|Viewport|AddtoViewport (Variables|Default|GetDewpercentWidgetBp) 0))))

(fn ConstructionScript)