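; Interactable object Blueprint that shows a widget while the player character is inside its trigger box and can move by a set offset.
; Tick rotates a Scene component to face the player every frame.
; The Start event plays a timeline that lerps the root from its current location to that point plus ENDLocation.
; The Stop event and leaving the box both halt the timeline and snap the root back, with overlap exit also hiding the widget.
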(event OnComponentBeginOverlap(Box)
  (params (OverlappedComponent :type Primitive%20Component%20Object%20Reference) (OtherActor :type Actor%20Object%20Reference) (OtherComp :type Primitive%20Component%20Object%20Reference) (OtherBodyIndex :type Integer) (bFromSweep :type Boolean) (SweepResult :type Hit%20Result%20Structure%20%28by%20ref%29))
  (Utilities|Casting|CastToBP_ThirdPersonCharacter1010 OtherActor)
  (Rendering|SetVisibility (Variables|Default|GetWidget) true false))

(event OnComponentEndOverlap(Box)
  (params (OverlappedComponent :type Primitive%20Component%20Object%20Reference) (OtherActor :type Actor%20Object%20Reference) (OtherComp :type Primitive%20Component%20Object%20Reference) (OtherBodyIndex :type Integer))
  (bind _start_location (Variables|Default|GetStart%20Location))
  (Utilities|Casting|CastToBP_ThirdPersonCharacter1010 OtherActor)
  (Rendering|SetVisibility (Variables|Default|GetWidget) false false)
  (Utilities|FlowControl|Sequence
    (:then_0
      (bind _newtrack_0 (Timeline|Movement Stop)
        (:Update
          (Transformation|SetWorldLocation (Variables|Default|GetDefaultSceneRoot) (Math|Vector|Lerp(Vector) _start_location (+ _start_location (Variables|Default|GetEND%20Location)) _newtrack_0) false false))))
    (:then_1
      (Transformation|SetWorldLocation (Variables|Default|GetDefaultSceneRoot) (Variables|Default|GetStart%20Location) false false))))

(event Custom|Start
  (Variables|Default|SetStart%20Location (Transformation|GetWorldLocation (Variables|Default|GetDefaultSceneRoot)))
  (bind _newtrack_0 (Timeline|Movement Play)
    (:Update
      (Transformation|SetWorldLocation (Variables|Default|GetDefaultSceneRoot) (Math|Vector|Lerp(Vector) (Variables|Default|GetStart%20Location) (+ (Variables|Default|GetStart%20Location) (Variables|Default|GetEND%20Location)) _newtrack_0) false false))))

(event Custom|Stop
  (bind _start_location (Variables|Default|GetStart%20Location))
  (Utilities|FlowControl|Sequence
    (:then_0
      (bind _newtrack_0 (Timeline|Movement Stop)
        (:Update
          (Transformation|SetWorldLocation (Variables|Default|GetDefaultSceneRoot) (Math|Vector|Lerp(Vector) _start_location (+ _start_location (Variables|Default|GetEND%20Location)) _newtrack_0) false false))))
    (:then_1
      (Transformation|SetWorldLocation (Variables|Default|GetDefaultSceneRoot) (Variables|Default|GetStart%20Location) false false))))

(event EventTick
  (params (DeltaSeconds :type Float%20%28single-precision%29))
  (Transformation|SetWorldRotation (Variables|Default|GetScene) (Math|Rotator|FindLookatRotation (Transformation|GetWorldLocation (Variables|Default|GetScene)) (Transformation|GetActorLocation (Game|GetPlayerCharacter 0))) false false))

(fn ConstructionScript)