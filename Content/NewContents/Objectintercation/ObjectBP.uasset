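; Interactable object Blueprint that shows a widget when the player character is in range and moves its cube when Interact is called.
; Box overlaps toggle the widget's visibility for BP_ThirdPersonCharacter1010.
; Interact plays the UPDONW timeline to lerp the cube from its current location by the ENDLocation offset, and leaving the box stops it and resets the cube.
; Tick rotates the Scene component to face the player.
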(event OnComponentBeginOverlap(Box)
  (params (OverlappedComponent :type Primitive%20Component%20Object%20Reference) (OtherActor :type Actor%20Object%20Reference) (OtherComp :type Primitive%20Component%20Object%20Reference) (OtherBodyIndex :type Integer) (bFromSweep :type Boolean) (SweepResult :type Hit%20Result%20Structure%20%28by%20ref%29))
  (Utilities|Casting|CastToBP_ThirdPersonCharacter1010 OtherActor)
  (Rendering|SetVisibility (Variables|Default|GetWidget) true false))

(event OnComponentEndOverlap(Box)
  (params (OverlappedComponent :type Primitive%20Component%20Object%20Reference) (OtherActor :type Actor%20Object%20Reference) (OtherComp :type Primitive%20Component%20Object%20Reference) (OtherBodyIndex :type Integer))
  (Utilities|Casting|CastToBP_ThirdPersonCharacter1010 OtherActor)
  (Rendering|SetVisibility (Variables|Default|GetWidget) false false)
  (CallFunction|Stop))

(event Custom|Stop
  (Utilities|FlowControl|Sequence
    (:then_0
      (bind _newtrack_0 (Timeline|UPDONW Stop)
        (:Update
          (Transformation|SetWorldLocation (Variables|Default|GetCube) (Math|Vector|Lerp(Vector) (Variables|Default|GetStart%20Location) (+ (Variables|Default|GetStart%20Location) (Variables|Default|GetEND%20Location)) _newtrack_0) false false))))
    (:then_1
      (Transformation|SetRelativeLocation (Variables|Default|GetCube) "0, 0, 0" false false))))

(event EventInteract
  (Rendering|SetVisibility (Variables|Default|GetWidget) true false)
  (Variables|Default|SetStart%20Location (Transformation|GetWorldLocation (Variables|Default|GetCube)))
  (bind _newtrack_0 (Timeline|UPDONW Play)
    (:Update
      (Transformation|SetWorldLocation (Variables|Default|GetCube) (Math|Vector|Lerp(Vector) (Variables|Default|GetStart%20Location) (+ (Variables|Default|GetStart%20Location) (Variables|Default|GetEND%20Location)) _newtrack_0) false false))))

(event EventTick
  (params (DeltaSeconds :type Float%20%28single-precision%29))
  (Transformation|SetWorldRotation (Variables|Default|GetScene) (Math|Rotator|FindLookatRotation (Transformation|GetWorldLocation (Variables|Default|GetScene)) (Transformation|GetActorLocation (Game|GetPlayerCharacter 0))) false false))

(fn ConstructionScript)